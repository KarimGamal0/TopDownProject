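; Enemy character Blueprint that chases the player and plays an attack animation when it gets close.
; Actor overlap with a CharacterMovement_BP sets the in-range flag and starts an AIMoveTo toward the player; ending overlap clears it and stops movement immediately.
; Reaching the player plays the attack montage, gated by an AttackRate cooldown.
; Montage completion resumes the chase if still in range, while arrivals during cooldown re-issue it directly.
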(event `self.ReceiveActorBeginOverlap`
  (params (OtherActor :type "Actor Object Reference"))
  (cast `/Game/Blueprints/CharacterMovement_BP` OtherActor)
  (set `self.PlayerInRange` true)
  (`self.Chase Player`))

(event `self.ReceiveActorEndOverlap`
  (params (OtherActor :type "Actor Object Reference"))
  (cast `/Game/Blueprints/CharacterMovement_BP` OtherActor)
  (set `self.PlayerInRange` false)
  (`MovementComponent.StopMovementImmediately` (`self.CharacterMovement`)))

(event `Chase Player`
  (`|AIMoveTo` self (0.0 0.0 0.0) (`GameplayStatics.GetPlayerCharacter` 0) 100.0
    (:`OnSuccess`
      (if (`self.CanAttack`)
        (set `self.CanAttack` false)
        (`|PlayMontage` (`self.Mesh`) "/Game/Enemy/Enemy_Attack_BP.Enemy_Attack_BP"
          (:`then`
            (`KismetSystemLibrary.Delay` (`self.AttackRate`))
            (set `self.CanAttack` true))
          (:`OnCompleted`
            (if (`self.PlayerInRange`)
              (`self.Chase Player`))))
        (else
          (`self.Chase Player`))))))

(fn `UserConstructionScript`)