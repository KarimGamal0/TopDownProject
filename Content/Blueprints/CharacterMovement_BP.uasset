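; Character Blueprint that handles a sword attack input, rooting the character in place during the slash.
; Pressing Attack, when no slash is active, stops and disables movement and sets the SlashSword flag.
; After a fixed delay it clears the flag and restores walking, so the flag also blocks repeated attacks until then.
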(event `InputAction|Attack`
  (params (Key :type "Key Structure"))
  (:`Pressed`
    (if (not (`self.SlashSword`))
      (`CharacterMovementComponent.DisableMovement` (`self.CharacterMovement`))
      (`MovementComponent.StopMovementImmediately` (`self.CharacterMovement`))
      (set `self.SlashSword` true)
      (`KismetSystemLibrary.Delay` 6.0)
      (set `self.SlashSword` false)
      (`CharacterMovementComponent.SetMovementMode` (`self.CharacterMovement`) "MOVE_Walking" 0))))

(fn `UserConstructionScript`)